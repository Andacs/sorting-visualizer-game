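; BP_SortingManager is the manager for a sorting visualizer: it spawns bars with random values and defines a bubble sort over them.
; BeginPlay spawns a row of BP_Bar actors and calls UpdateBar on each, but the node adding them to Bars is unconnected.
; BubbleSort uses nested loops to compare BarValue and swap array entries only, without moving actors, then prints a completion message.
; Nothing in this Blueprint calls BubbleSort.
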(event `BubbleSort`
  (bind _bars (`self.Bars`))
  (bind _returnvalue (`KismetArrayLibrary.Array_Length` _bars))
  (for _index (range _returnvalue)
    (for _index_2 (range (- _returnvalue _index))
      (bind _returnvalue_2 (+ _index_2 1))
      (if (> (`/Game/SortingVisualizer/Blueprints/BP_Bar.BarValue` (`|GetArrayItem` _bars _index_2)) (`/Game/SortingVisualizer/Blueprints/BP_Bar.BarValue` (`|GetArrayItem` _bars _returnvalue_2)))
        (`KismetArrayLibrary.Array_Swap` _bars _index_2 _returnvalue_2))))
  (`KismetSystemLibrary.PrintString` "sıralama bitti"))

(event `self.ReceiveBeginPlay`
  (for _index (range (`self.NumBars`))
    (bind _returnvalue (`|SpawnActorFromClass` "/Game/SortingVisualizer/Blueprints/BP_Bar.BP_Bar_C" (`KismetMathLibrary.MakeTransform` (`KismetMathLibrary.MakeVector` (* _index (`self.BarSpacing`)) 0.0 200.0)) "Undefined" "MultiplyWithRoot" null null))
    (set `/Game/SortingVisualizer/Blueprints/BP_Bar.BarValue` (`KismetMathLibrary.RandomIntegerInRange` (`self.MinValue`) (`self.MaxValue`)) _returnvalue)
    (`/Game/SortingVisualizer/Blueprints/BP_Bar.UpdateBar` _returnvalue)))

(fn `UserConstructionScript`)